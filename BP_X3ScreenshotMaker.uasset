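; BP_X3ScreenshotMaker is a placeable camera actor that saves timestamped JPG screenshots to an export path, manually or on a timer.
; BeginPlay creates a viewport-sized render target for its SceneCaptureComponent2D and, when new, defaults the camera to 3 m above the actor.
; UpdateCamPosition applies the stored camera transform, and TakeScreenshot captures and exports the image.
; StartAutoScreenshot starts the looping capture timer if enabled and absent, otherwise clearing any existing one.
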(event EventBeginPlay
  (bind _returnvalue (Viewport|GetViewportSize))
  (bind _returnvalue_2 (Transformation|GetActorLocation))
  (bind _returnvalue_3 (Rendering|CreateRenderTarget2D (Math|Float|Truncate (.x _returnvalue)) (Math|Float|Truncate (.y _returnvalue)) "RTF_RGBA8"))
  (bind _output_get (Variables|Default|SetRenderTarget2D _returnvalue_3))
  (Variables|/Script/Engine.TextureRenderTarget|SetTargetGamma _output_get 0.02)
  (Variables|/Script/Engine.SceneCaptureComponent2D|SetTextureTarget (Variables|Default|GetSceneCaptureComponent2D1) (Variables|Default|GetRenderTarget2D))
  (if (Variables|Default|GetIsNew)
    ;[1 1 1] Set current camera position to vars (default values)
    (Variables|Default|SetCamLocation (Math|Vector|MakeVector (.x _returnvalue_2) (.y _returnvalue_2) (+ (.z _returnvalue_2) 3e+02)))
    (Variables|Default|SetCamRotation (Transformation|GetActorRotation)))
  ;[1 1 1] Update Cam & take Screenshot
  (CallFunction|UpdateCamPosition)
  (CallFunction|StartAutoScreenshot))

(event Collision|EventActorBeginOverlap
  (params (OtherActor :type Actor%20Object%20Reference)))

(fn ConstructionScript)

(fn DEBUG(SM)
  (params (DebugMessage :type String))
  (Class|SMLPlayerComponent|SendChatMessage (Actor|GetComponentbyClass (Game|GetPlayerController 0) "/Script/SML.SMLPlayerComponent") DebugMessage (LocalVariables|GetColor)))

(fn TakeScreenshot
  (bind _returnvalue (Math|DateTime|Now))
  ;[1 1 1] Capture
  (Rendering|SceneCapture|CaptureScene (Variables|Default|GetSceneCaptureComponent2D1) :!class /Script/Engine.SceneCaptureComponent2D)
  ;[1 1 1] Save to file
  (Class|ImageWriteBlueprintLibrary|ExporttoDisk (Variables|Default|GetRenderTarget2D) (Utilities|String|Append (Utilities|String|Append (Variables|Default|GetExportPath) "\\X3_") (Utilities|String|ToString(Integer) (Class|KismetMathLibrary|GetYear _returnvalue)) "_" (Utilities|String|ToString(Integer) (Class|KismetMathLibrary|GetMonth _returnvalue)) "_" (Utilities|String|ToString(Integer) (Class|KismetMathLibrary|GetDay _returnvalue)) "__" (Utilities|String|ToString(Integer) (Class|KismetMathLibrary|GetHour _returnvalue)) "_" (Utilities|String|ToString(Integer) (Class|KismetMathLibrary|GetMinute _returnvalue)) "_" (Utilities|String|ToString(Integer) (Class|KismetMathLibrary|GetSecond _returnvalue)) "_" (Utilities|String|ToString(Integer) (Math|DateTime|GetMillisecond _returnvalue)) ".jpg") (Utilities|Struct|MakeImageWriteOptions "JPG" (EventDispatchers|CreateEvent :!event OnScreenshotComplete) 75)))

(fn OnScreenshotComplete
  (params (NewParam :type Boolean)))

(fn UpdateCamPosition
  (Variables|Default|SetIsNew false)
  (Transformation|SetWorldLocationAndRotation (Variables|Default|GetSceneCaptureComponent2D1) (Variables|Default|GetCamLocation) (Variables|Default|GetCamRotation) false true))

(fn StartAutoScreenshot
  (if (and (Variables|Default|GetAutoEnabled) (not (Class|KismetSystemLibrary|TimerExists 0 "TakeScreenshot"))) ; Is enabled AND timer does NOT exists?
    (Utilities|Time|SetTimerbyFunctionName 0 "TakeScreenshot" (Variables|Default|GetAutoSeconds) true)
    (elif (Class|KismetSystemLibrary|TimerExists 0 "TakeScreenshot") ; Else (if timer exists)
      (Utilities|Time|ClearTimerbyFunctionName 0 "TakeScreenshot"))))